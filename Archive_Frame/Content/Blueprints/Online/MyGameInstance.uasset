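; Game instance Blueprint that provides events to host, find, join and destroy LAN multiplayer sessions.
; Hosting creates a session with zero public connections, then runs a debug search that prints the found server's name.
; FindSession stores FoundSessions from the async node's immediate output rather than its success callback.
; JoinSession takes the first stored result without checking that any exist.
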(event Custom|HostSession
  (bind _returnvalue (Game|GetPlayerController 0))
  (|Session _returnvalue 0 true
    (:OnSuccess
      (Development|PrintString "Session Made, Stop Clicking")
      (bind _results (|FindSessions _returnvalue 1 true)
        (:OnSuccess
          (Development|PrintString (Class|FindSessionsCallbackProxy|GetServerName (Utilities|Array|Get(acopy) _results))))))))

(event Custom|FindSession
  (bind _results (|FindSessions (Game|GetPlayerController 0) 10 true)
    (:then
      (Variables|Default|SetFoundSessions _results))))

(event Custom|JoinSession
  (|JoinSession (Game|GetPlayerController 0) (Utilities|Array|Get(acopy) (Variables|Default|GetFoundSessions))))

(event Custom|DestoryGame
  (|DestroySession (Game|GetPlayerController 0)))